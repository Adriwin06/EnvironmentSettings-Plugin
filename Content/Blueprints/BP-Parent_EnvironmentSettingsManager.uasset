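; Parent environment settings manager that drives color cube grading, vignette and bloom post-processing from the time of day.
; Time changes fetch the two surrounding EnvironmentTimeline keyframes and a blend factor.
; These feed two LUT textures and a blend to the color cube's dynamic material, and lerped values to a Material Parameter Collection and bloom threshold.
; The construction script applies the blend and per-effect dev toggles, which set blendable weights by index.
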(event Custom|ToggleEffects
  ;[0.15 0.15 0.15 0.5] Dev Toggles
  (CallFunction|ToggleColorCube (Variables|EditorToggles|GetbEnableColorCube))
  (CallFunction|ToggleVignette (Variables|EditorToggles|GetbEnableVignette))
  (CallFunction|ToggleBloom (Variables|EditorToggles|GetbEnableBloom)))

(event Custom|ToggleColorCube
  (params (Enabled :type Boolean))
  ;[0.15 0.15 0.15 0.5] Dev Toggles
  (bind _output_get (Variables|EditorToggles|SetbEnableColorCube Enabled))
  (EffectsToggle|TogglePostProcessMaterial (Variables|Default|GetPostProcess) _output_get))

(event Custom|KeyframesBlending
  (params (TimeOfDay :type Float%20%28double-precision%29))
  (bind _environmenttimeline (Variables|Environment|GetEnvironmentTimeline))
  (bind (_keyframebefore _keyframeafter _blendfactor) (Class|EnvironmentStatics|GetEnvironmentKeyframesforTime _environmenttimeline TimeOfDay))
  (bind _output_get (Variables|Environment|SetTimeOfDay_Seconds TimeOfDay))
  (Variables|EditorToggles|SetTimeOfDay (Utilities|CalculateTimeOfDay _output_get))
  (Variables|Environment|SetEnvironmentKeyframe_Before _keyframebefore)
  (Variables|Environment|SetEnvironmentKeyframe_After _keyframeafter)
  (Variables|Environment|SetBlendFactor _blendfactor)
  (CallFunction|UpdatePostProcess))

(event Custom|ToggleVignette
  (params (Enabled :type Boolean))
  ;[0.15 0.15 0.15 0.5] Dev Toggles
  (bind _output_get (Variables|EditorToggles|SetbEnableVignette Enabled))
  (EffectsToggle|TogglePostProcessMaterial (Variables|Default|GetPostProcess) _output_get 1))

(event Custom|UpdatePostProcess
  (UpdatePostProcess|UpdateVignette)
  (UpdatePostProcess|UpdateColorCube)
  (UpdatePostProcess|UpdateBloom))

(event Custom|ToggleBloom
  (params (Enabled :type Boolean))
  ;[0.15 0.15 0.15 0.5] Dev Toggles
  (bind _output_get (Variables|EditorToggles|SetbEnableBloom Enabled))
  (EffectsToggle|TogglePostProcessMaterial (Variables|Default|GetPostProcess) _output_get 2))

(event Custom|Initializations
  (CallFunction|InitializeMaterialInstances)
  (CallFunction|SetPostProcessMaterials (Variables|Default|GetPostProcess) (Variables|Materials|GetDMIs)))

(event EventBeginPlay
  (CallFunction|Initializations))

(event EventTimeofDayChange
  (params (TimeOfDay :type Float%20%28double-precision%29))
  (CallFunction|KeyframesBlending TimeOfDay))

(fn ConstructionScript
  (CallFunction|Initializations)
  (CallFunction|ToggleEffects)
  (bind _output_get (Variables|Environment|SetTimeOfDay_Seconds (Utilities|CalculateTimeOfDaySeconds (Variables|EditorToggles|GetTimeOfDay))))
  (CallFunction|KeyframesBlending _output_get))

(fn InitializeMaterialInstances
  (bind (_keypin _valuepin) (Utilities|Map|ForEachLoop(Map) (Variables|Materials|GetParentMaterials))
    (:then
      (bind _returnvalue (Rendering|Material|CreateDynamicMaterialInstance _valuepin "None" "None" :!class /Script/Engine.KismetMaterialLibrary))
      (Utilities|Map|Add (Variables|Materials|GetDMIs) _keypin _returnvalue))))

(fn SetPostProcessMaterials
  (params (PostProcessComp :type Post%20Process%20Component%20Object%20Reference) (DynamicMaterialInstances :type Map%20of%20Strings%20to%20Objects))
  (bind _valuepin (Utilities|Map|ForEachLoop(Map) DynamicMaterialInstances)
    (:then
      (Utilities|Array|Add (LocalVariables|GetWeightedBlendables) (Utilities|Struct|MakeWeightedBlendable 1.0 _valuepin)))
    (:CompletedPin
      (Variables|/Script/Engine.PostProcessComponent|SetSettings PostProcessComp (Utilities|Struct|MakePostProcessSettings (Utilities|Struct|MakeWeightedBlendables (LocalVariables|GetWeightedBlendables)))))))

(fn UpdateVignette
  (Utilities|FlowControl|Sequence
    (:then_0
      (Utilities|UpdateScalarMPC (Variables|/Script/EnvironmentSettings.EnvironmentKeyframeData|GetVignetteAngle (Variables|Environment|GetEnvironmentKeyframe_Before)) (Variables|/Script/EnvironmentSettings.EnvironmentKeyframeData|GetVignetteAngle (Variables|Environment|GetEnvironmentKeyframe_After)) "Vignette_RotationAngle"))
    (:then_1
      (Utilities|UpdateScalarMPC (Variables|/Script/EnvironmentSettings.EnvironmentKeyframeData|GetVignetteSharpness (Variables|Environment|GetEnvironmentKeyframe_Before)) (Variables|/Script/EnvironmentSettings.EnvironmentKeyframeData|GetVignetteSharpness (Variables|Environment|GetEnvironmentKeyframe_After)) "Vignette_Sharpness"))
    (:then_2
      (Utilities|UpdateVector2MPC (Variables|/Script/EnvironmentSettings.EnvironmentKeyframeData|GetVignetteAmount (Variables|Environment|GetEnvironmentKeyframe_Before)) (Variables|/Script/EnvironmentSettings.EnvironmentKeyframeData|GetVignetteAmount (Variables|Environment|GetEnvironmentKeyframe_After)) "Vignette_Size"))
    (:then_3
      (Utilities|UpdateVector2MPC (Variables|/Script/EnvironmentSettings.EnvironmentKeyframeData|GetVignetteCenter (Variables|Environment|GetEnvironmentKeyframe_Before)) (Variables|/Script/EnvironmentSettings.EnvironmentKeyframeData|GetVignetteCenter (Variables|Environment|GetEnvironmentKeyframe_After)) "Vignettte_CenterPosition"))
    (:then_4
      (Utilities|UpdateLinearColorMPC (Variables|/Script/EnvironmentSettings.EnvironmentKeyframeData|GetVignetteInnerColor (Variables|Environment|GetEnvironmentKeyframe_Before)) (Variables|/Script/EnvironmentSettings.EnvironmentKeyframeData|GetVignetteInnerColor (Variables|Environment|GetEnvironmentKeyframe_After)) "Vignette_InnerColor"))
    (:then_5
      (Utilities|UpdateLinearColorMPC (Variables|/Script/EnvironmentSettings.EnvironmentKeyframeData|GetVignetteOuterColor (Variables|Environment|GetEnvironmentKeyframe_Before)) (Variables|/Script/EnvironmentSettings.EnvironmentKeyframeData|GetVignetteOuterColor (Variables|Environment|GetEnvironmentKeyframe_After)) "Vignette_OuterColor"))))

(fn UpdateColorCube
  (bind _dmis (Variables|Materials|GetDMIs))
  (bind _value (Utilities|Map|Find _dmis "ColorCube"))
  (Rendering|Material|SetTextureParameterValue _value "LUT_Texture_A" (Variables|/Script/EnvironmentSettings.EnvironmentKeyframeData|GetColorCubeReference (Variables|Environment|GetEnvironmentKeyframe_Before)))
  (Rendering|Material|SetTextureParameterValue _value "LUT_Texture_B" (Variables|/Script/EnvironmentSettings.EnvironmentKeyframeData|GetColorCubeReference (Variables|Environment|GetEnvironmentKeyframe_After)))
  (Rendering|Material|SetScalarParameterValue _value "LUT_Blend" (Variables|Environment|GetBlendFactor) :!class /Script/Engine.MaterialInstanceDynamic))

(fn UpdateBloom
  (Utilities|UpdateScalarMPC (Variables|/Script/EnvironmentSettings.EnvironmentKeyframeData|GetBloomLuminance (Variables|Environment|GetEnvironmentKeyframe_Before)) (Variables|/Script/EnvironmentSettings.EnvironmentKeyframeData|GetBloomLuminance (Variables|Environment|GetEnvironmentKeyframe_After)) "Bloom_Luminance")
  (Utilities|UpdateVector4MPC (Variables|/Script/EnvironmentSettings.EnvironmentKeyframeData|GetBloomScale (Variables|Environment|GetEnvironmentKeyframe_Before)) (Variables|/Script/EnvironmentSettings.EnvironmentKeyframeData|GetBloomScale (Variables|Environment|GetEnvironmentKeyframe_After)) "Bloom_Scale")
  (bind _structout (Utilities|Struct|SetmembersinPostProcessSettings (Variables|/Script/Engine.PostProcessComponent|GetSettings (Variables|Default|GetPostProcess)) (Math|Float|Lerp (Variables|/Script/EnvironmentSettings.EnvironmentKeyframeData|GetBloomThreshold (Variables|Environment|GetEnvironmentKeyframe_Before)) (Variables|/Script/EnvironmentSettings.EnvironmentKeyframeData|GetBloomThreshold (Variables|Environment|GetEnvironmentKeyframe_After)) (Variables|Environment|GetBlendFactor))))
  (Variables|/Script/Engine.PostProcessComponent|SetSettings (Variables|Default|GetPostProcess) _structout))

(fn TogglePostProcessMaterial
  (params (PostProcesComponent :type Post%20Process%20Component%20Object%20Reference) (bEnabled :type Boolean) (MaterialIndex :type Integer))
  (for (_array_element _array_index) (Utilities|Struct|BreakWeightedBlendables (Utilities|Struct|BreakPostProcessSettings (Variables|/Script/Engine.PostProcessComponent|GetSettings PostProcesComponent)))
    (if (== _array_index MaterialIndex)
      (Utilities|Array|Add (LocalVariables|GetPostProcessMaterials) (Utilities|Struct|MakeWeightedBlendable (Math|Conversions|ToFloat(Boolean) bEnabled) (.Object (Utilities|Struct|BreakWeightedBlendable _array_element))))
      (else
        (Utilities|Array|Add (LocalVariables|GetPostProcessMaterials) _array_element))))
  (Variables|/Script/Engine.PostProcessComponent|SetSettings PostProcesComponent (Utilities|Struct|MakePostProcessSettings (Utilities|Struct|MakeWeightedBlendables (LocalVariables|GetPostProcessMaterials)))))